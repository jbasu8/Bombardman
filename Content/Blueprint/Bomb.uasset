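; Bomb actor for a Bomberman-style game that explodes three seconds after spawning and then destroys itself.
; On detonation it decrements the Bombs count on every Player1 actor.
; It then checks Sphere1 overlaps, destroying any Player1 or Player2 and calling DropChance on BreakableBlocks before destroying them.
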(event `self.ReceiveBeginPlay`
  (`KismetSystemLibrary.Delay` 3.0)
  (bind _outactors (`GameplayStatics.GetAllActorsOfClass` "/Game/Blueprint/Player1.Player1_C"))
  (for _array_element _outactors
    (`/Engine/EditorBlueprintResources/StandardMacros.DecrementInt` (`/Game/Blueprint/Player1.bombs` _array_element)))
  (bind _output_get (set `self.NewVar_0` (`PrimitiveComponent.GetOverlappingActors` (`self.Sphere1`) null)))
  (for _array_element_2 _output_get
    (bind _returnvalue (`GameplayStatics.GetObjectClass` _array_element_2))
    (if (or (== _returnvalue "/Game/Blueprint/Player1.Player1_C") (== _returnvalue "/Game/Blueprint/Player2.Player2_C"))
      (`self.K2_DestroyActor` _array_element_2)
      (elif (== _returnvalue "/Game/Blueprint/BreakableBlock.BreakableBlock_C")
        (bind _asbreakable_block (cast `/Game/Blueprint/BreakableBlock` _array_element_2))
        (`/Game/Blueprint/BreakableBlock.drop chance` _asbreakable_block)
        (`self.K2_DestroyActor` _array_element_2))))
  (`self.K2_DestroyActor`))

(fn `UserConstructionScript`)