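; Bomb_2 is Player 2's bomb in what appears to be a Bomberman-style game.
; On BeginPlay it waits through a fuse delay, then decrements the Bombs count on every Player2 actor.
; An unconnected blast chain, which never runs, would destroy players and BreakableBlocks overlapping Sphere1, calling DropChance on blocks first, then destroy the bomb itself.
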(event `self.ReceiveBeginPlay`
  (`KismetSystemLibrary.Delay` 3.0)
  (bind _outactors (`GameplayStatics.GetAllActorsOfClass` "/Game/Blueprint/Player2.Player2_C"))
  (for _array_element _outactors
    (`/Engine/EditorBlueprintResources/StandardMacros.DecrementInt` (`/Game/Blueprint/Player2.bombs` _array_element))))

(fn `UserConstructionScript`)