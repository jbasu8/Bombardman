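; Player2 is the second player's Blueprint, a physics-driven cube that moves and drops bombs.
; Each Tick pushes the Cube along X and Y using the Forward2 and Right2 values, applied as mass-independent acceleration.
; Pressing Enter spawns a Bomb_2 above the cube unless Bombs equals Maxbombs; the count is not changed in this graph.
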(event `self.ReceiveTick`
  (params (DeltaSeconds :type "Float (single-precision)"))
  (`PrimitiveComponent.AddForce` (`self.Cube`) (`KismetMathLibrary.MakeVector` (* (`self.GetInputAxisValue`) 10000.0) (* (`self.GetInputAxisValue`) 10000.0)) "None" true))

(event `Key|Enter`
  (params (Key :type "Key Structure"))
  (:`Pressed`
    (if (!= (`self.bombs`) (`self.maxbombs`))
      (`|SpawnActorFromClass` "/Game/Blueprint/Bomb_2.Bomb_2_C" (`KismetMathLibrary.Conv_VectorToTransform` (`KismetMathLibrary.MakeVector` (.x (`SceneComponent.K2_GetComponentLocation` (`self.Cube`))) (.y (`SceneComponent.K2_GetComponentLocation` (`self.Cube`))) (+ (.z (`SceneComponent.K2_GetComponentLocation` (`self.Cube`))) 250.0))) "Undefined" "OverrideRootScale" null null))))

(fn `UserConstructionScript`)